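; BP_Missile is a projectile for the Level 4 lock-on shooting content that can home on a target actor.
; BeginPlay launches it forward at combined initial and base speed, then after a short delay enables sphere collision and assigns the movement component's homing target if ShouldHome is set.
; On hit it destroys itself and any BP_Enemy_Test_Shooting it struck, with debug prints.
; The node enabling IsHomingProjectile is unwired.
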(event `self.ReceiveBeginPlay`
  (bind _returnvalue (`self.GetInstigator`))
  (set `MovementComponent.Velocity` (* (+ (`self.InitialSpeed`) (`self.BaseSpeed`)) (`self.GetActorForwardVector`)) (`self.ProjectileMovement`))
  (`KismetSystemLibrary.Delay` 0.1)
  (`PrimitiveComponent.SetCollisionEnabled` (`self.SphereCollsion`) "QueryAndPhysics")
  (`KismetSystemLibrary.PrintString` (`KismetSystemLibrary.GetDisplayName` _returnvalue) false)
  (`PrimitiveComponent.IgnoreActorWhenMoving` (`self.SphereCollsion`) _returnvalue false)
  (if (`self.shouldHome`)
    (set `ProjectileMovementComponent.HomingTargetComponent` (`Actor.RootComponent` (`self.TargetActor`)) (`self.ProjectileMovement`))))

(event `self.ReceiveHit`
  (params (MyComp :type "PrimitiveComponent Object Reference") (Other :type "Actor Object Reference") (OtherComp :type "PrimitiveComponent Object Reference") (bSelfMoved :type Boolean) (HitLocation :type "Vector Structure") (HitNormal :type "Vector Structure") (NormalImpulse :type "Vector Structure") (Hit :type "HitResult Structure (by ref)"))
  (`KismetSystemLibrary.PrintString` (`KismetSystemLibrary.GetDisplayName` Other) true true (struct :`R` 1.0 :`G` 0.182047 :`A` 1.0))
  (bind _asbp_enemy_test_shooting (cast `/Game/Content_Level4/EnemyCharacter_Level4/BasicEnemy/BP_Enemy_Test_Shooting` Other)
    (:`then`
      (`self.K2_DestroyActor` _asbp_enemy_test_shooting))
    (:`CastFailed`
      _))
  (`self.K2_DestroyActor`)
  (`KismetSystemLibrary.PrintString` "Missle collision event"))

(fn `UserConstructionScript`)