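; Level 4 game mode Blueprint that tracks how many outposts remain.
; On BeginPlay it seeds OutpostsRemaining from the count returned by GetAllActorsOfClass.
; Each OutpostDestroyed event decrements the counter, and at zero or below it prints a boss-spawn message as a placeholder, with no actual spawn logic.
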(event `self.ReceiveBeginPlay`
  (bind _outactors (`GameplayStatics.GetAllActorsOfClass` null))
  (set `self.OutpostsRemaining` (`KismetArrayLibrary.Array_Length` _outactors)))

(event `OutpostDestroyed`
  (set `self.OutpostsRemaining` (- (`self.OutpostsRemaining`) 1))
  (if (<= (`self.OutpostsRemaining`) 0)
    (`KismetSystemLibrary.PrintString` "SPAWN THE BOSS!")))

(fn `UserConstructionScript`)