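; Level 4 game mode that runs three combat stages in order as the player's airplane enters trigger areas.
; Each stage fires its spawners and resets HUD targets; registered enemy lists feed the radar.
; Meeting both aircraft and base kill targets clears remaining aircraft and unlocks the next trigger.
; In stage three, base kills trigger the mothership cannon sequence, ending in its crash, and full clearance fades out as the win.
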(event `self.ReceiveBeginPlay`
  ;[1 1 1] bind area enter
  (bind _outactors (`GameplayStatics.GetAllActorsOfClass` "/Game/Level4/Trigger_Volume/Trigger_Combat1.Trigger_Combat1_C"))
  (add `/Game/Level4/Trigger_Volume/Trigger_Combat1.EnterArea` (`|GetArrayItem` _outactors) (delegate `EnterCombat1`))
  (bind _outactors_2 (`GameplayStatics.GetAllActorsOfClass` "/Game/Level4/Trigger_Volume/Trigger_Combat2.Trigger_Combat2_C"))
  (add `/Game/Level4/Trigger_Volume/Trigger_Combat2.EnterArea` (`|GetArrayItem` _outactors_2) (delegate `EnterCombat2`))
  (bind _outactors_3 (`GameplayStatics.GetAllActorsOfClass` "/Game/Level4/Trigger_Volume/Trigger_End.Trigger_End_C"))
  (add `/Game/Level4/Trigger_Volume/Trigger_End.EnterArea` (`|GetArrayItem` _outactors_3) (delegate `EnterEnd`)))

(event `EnterEnd`
  (params (TriggerActor :type "Actor Object Reference"))
  ;[1 1 1] bind area enter
  (if (and (== (`GameplayStatics.GetObjectClass` TriggerActor) "/Game/JetPlaneMap/Blueprints/BP_Airplane.BP_Airplane_C") (`self.CanEnterNextProgress`) (== (`self.PlayerProgress`) 2))
    (`self.Update Game State`)
    (`KismetSystemLibrary.PrintString` "combat3")))

(event `EnterCombat1`
  (params (TriggerActor :type "Actor Object Reference"))
  ;[1 1 1] bind area enter
  (if (and (== (`GameplayStatics.GetObjectClass` TriggerActor) "/Game/JetPlaneMap/Blueprints/BP_Airplane.BP_Airplane_C") (`self.CanEnterNextProgress`) (== (`self.PlayerProgress`) 0))
    (`self.Update Game State`)
    (`KismetSystemLibrary.PrintString` "combat1")
    (bind _outactors (`GameplayStatics.GetAllActorsOfClass` "/Game/JetPlaneMap/Blueprints/BP_Airplane.BP_Airplane_C"))
    (message `/Game/Content_Level4/UI/Widgets/BPI_RaderManager.SetEnemyList` (`/Game/Content_Level4/UI/HUD/WBP_HUD_Main.WBP_RadarBase` (`/Game/JetPlaneMap/Blueprints/BP_Airplane.WBP_HUD_Main` (`|GetArrayItem` _outactors))) (`self.AntiAircraftEnemyList`) (`self.AircraftEnemyList`) (`self.BaseEnemyList`))))

(event `EnterCombat2`
  (params (TriggerActor :type "Actor Object Reference"))
  ;[1 1 1] bind area enter
  (if (and (== (`GameplayStatics.GetObjectClass` TriggerActor) "/Game/JetPlaneMap/Blueprints/BP_Airplane.BP_Airplane_C") (`self.CanEnterNextProgress`) (== (`self.PlayerProgress`) 1))
    (`self.Update Game State`)
    (`KismetSystemLibrary.PrintString` "combat2")))

(event `/Game/Content_Level4/EnemyCharacter_Level4/BasicEnemy/BPI_EnemyManager.EnemyDestroy`
  ;[1 1 1] aircraft enemy count
  (`KismetSystemLibrary.PrintString` "destroyed an enemy")
  (set `self.CurrentEstimate` (+ (`self.CurrentEstimate`) 1))
  (bind _outactors (`GameplayStatics.GetAllActorsOfClass` "/Game/JetPlaneMap/Blueprints/BP_Airplane.BP_Airplane_C"))
  (set `/Game/Content_Level4/UI/HUD/WBP_HUD_Main.AircraftsKilled` (`self.CurrentEstimate`) (`/Game/JetPlaneMap/Blueprints/BP_Airplane.WBP_HUD_Main` (`|GetArrayItem` _outactors)))
  (if (>= (`self.CurrentEstimate`) (`self.AircraftTargets`))
    (set `self.AircraftEnemyClear` true)
    (if (`self.BaseEnemyClear`)
      (`self.ClearEnemy`)
      (set `self.CanEnterNextProgress` true)
      (`self.UpdateUIText`)
      (if (== (`self.PlayerProgress`) 3)
        (`self.Win`)))))

(event `/Game/Content_Level4/EnemyCharacter_Level4/BasicEnemy/BPI_EnemyManager.RegisterEnemy`
  (params (CurrentEnemy :type "Pawn Object Reference"))
  ;[1 1 1] add enemy
  (`self.AddEnemy` CurrentEnemy))

(event `Win`
  ;[1 1 1] Win
  (`PlayerCameraManager.StartCameraFade` :`self` (`GameplayStatics.GetPlayerCameraManager` 0) :`ToAlpha` 1.0 :`Duration` 10.0 :`bShouldFadeAudio` true :`bHoldWhenFinished` true))

(event `/Game/Content_Level4/EnemyCharacter_Level4/BasicEnemy/BPI_EnemyManager.RemoveEnemy`
  (params (CurrentEnemy :type "Pawn Object Reference"))
  ;[1 1 1] remove enemy
  (`self.Remove Enemy` CurrentEnemy))

(event `/Game/Content_Level4/EnemyCharacter_Level4/BasicEnemy/BPI_EnemyManager.BaseEnemyDestroy`
  ;[1 1 1] base enemy count
  (`KismetSystemLibrary.PrintString` "destroyed a base")
  (if (== (`self.PlayerProgress`) 3)
    (`self.FireMotherShip`))
  (set `self.CurrentBaseEstimate` (+ (`self.CurrentBaseEstimate`) 1))
  (bind _outactors (`GameplayStatics.GetAllActorsOfClass` "/Game/JetPlaneMap/Blueprints/BP_Airplane.BP_Airplane_C"))
  (set `/Game/Content_Level4/UI/HUD/WBP_HUD_Main.BasesDestroyed` (`self.CurrentBaseEstimate`) (`/Game/JetPlaneMap/Blueprints/BP_Airplane.WBP_HUD_Main` (`|GetArrayItem` _outactors)))
  (if (>= (`self.CurrentBaseEstimate`) (`self.BaseTargets`))
    (if (== (`self.PlayerProgress`) 3)
      (set `self.GameOver` true))
    (set `self.BaseEnemyClear` true)
    (if (`self.AircraftEnemyClear`)
      (`self.ClearEnemy`)
      (set `self.CanEnterNextProgress` true)
      (`self.UpdateUIText`)
      (if (== (`self.PlayerProgress`) 3)
        (`self.Win`)))))

(event `/Game/Content_Level4/EnemyCharacter_Level4/BasicEnemy/BPI_EnemyManager.RegisterAntiAircraftEnemy`
  (params (CurrentEnemy :type "Pawn Object Reference"))
  ;[1 1 1] anti-aircraft enemy register
  (`self.AddAntiAircraft` CurrentEnemy))

(event `/Game/Content_Level4/EnemyCharacter_Level4/BasicEnemy/BPI_EnemyManager.RemoveAntiAircraftEnemy`
  (params (CurrentEnemy :type "Pawn Object Reference"))
  ;[1 1 1] anti-aircraft enemy remove
  (`self.RemoveAntiAircraft` CurrentEnemy))

(event `FireMotherShip`
  ;[1 1 1] Attack mother ship!!
  (bind _outactors (`GameplayStatics.GetAllActorsOfClass` "/Game/Content_Level4/EnemyCharacter_Level4/BasicEnemy/BP_EnemyBoss.BP_EnemyBoss_C"))
  (bind _output_get (set `self.MotherShip` (`|GetArrayItem` _outactors)))
  (`/Game/Content_Level4/EnemyCharacter_Level4/BasicEnemy/BP_EnemyBoss.CannonCharging` _output_get)
  (`KismetSystemLibrary.Delay` 5.0)
  (`/Game/Content_Level4/EnemyCharacter_Level4/BasicEnemy/BP_EnemyBoss.CannonFire` _output_get)
  (`KismetSystemLibrary.Delay` 1.0)
  (`/Game/Content_Level4/EnemyCharacter_Level4/BasicEnemy/BP_EnemyBoss.ExplodeBattleship` _output_get)
  (if (`self.GameOver`)
    (`/Game/Content_Level4/EnemyCharacter_Level4/BasicEnemy/BP_EnemyBoss.StartCrashBattleShip` _output_get)))

(event `self.ReceiveTick`
  (params (DeltaSeconds :type "Float (single-precision)"))
  ;[1 1 1] Attack mother ship!!
  (if (`self.GameOver`)
    (`/Game/Content_Level4/EnemyCharacter_Level4/BasicEnemy/BP_EnemyBoss.updateCrashBattleShip` (`self.MotherShip`) 0.0)))

(event `/Game/Content_Level4/EnemyCharacter_Level4/BasicEnemy/BPI_EnemyManager.RegisterBaseEnemy`
  (params (CurrentEnemy :type "Pawn Object Reference"))
  ;[1 1 1] base enemy register
  (`self.AddBase` CurrentEnemy))

(event `/Game/Content_Level4/EnemyCharacter_Level4/BasicEnemy/BPI_EnemyManager.RemoveBaseEnemy`
  (params (CurrentEnemy :type "Pawn Object Reference"))
  ;[1 1 1] base enemy remove
  (`self.RemoveBase` CurrentEnemy))

(fn `AddAntiAircraft`
  (params (CurrentEnemy :type "Pawn Object Reference"))
  (`KismetArrayLibrary.Array_Add` (`self.AntiAircraftEnemyList`) CurrentEnemy))

(fn `AddBase`
  (params (CurrentEnemy :type "Pawn Object Reference"))
  ;[1 1 1] add enemy instance
  (`KismetArrayLibrary.Array_Add` (`self.BaseEnemyList`) CurrentEnemy))

(fn `AddEnemy`
  (params (CurrentEnemy :type "Pawn Object Reference"))
  ;[1 1 1] add enemy instance
  (`KismetArrayLibrary.Array_Add` (`self.AircraftEnemyList`) CurrentEnemy))

(fn `ClearEnemy`
  ;[1 1 1] clear all enemy aircraft
  (for _array_element (`self.AircraftEnemyList`)
    (bind _asbp_enemy_aircraft (cast `/Game/Content_Level4/EnemyCharacter_Level4/BasicEnemy/BP_EnemyAircraft` _array_element))
    (`/Game/Content_Level4/EnemyCharacter_Level4/BasicEnemy/BP_EnemyAircraft.GetHit` _asbp_enemy_aircraft 99))
  (`KismetSystemLibrary.PrintString` "clear aircraft finished"))

(fn `Remove Enemy`
  (params (CurrentEnemy :type "Pawn Object Reference"))
  ;[1 1 1] remove current enemy
  (`KismetArrayLibrary.Array_RemoveItem` (`self.AircraftEnemyList`) CurrentEnemy))

(fn `RemoveAntiAircraft`
  (params (CurrentEnemy :type "Pawn Object Reference"))
  (bind _returnvalue (`KismetArrayLibrary.Array_RemoveItem` (`self.AntiAircraftEnemyList`) CurrentEnemy)))

(fn `RemoveBase`
  (params (CurrentEnemy :type "Pawn Object Reference"))
  (bind _returnvalue (`KismetArrayLibrary.Array_RemoveItem` (`self.BaseEnemyList`) CurrentEnemy)))

(fn `Update Game State`
  (bind _output_get (set `self.PlayerProgress` (+ (`self.PlayerProgress`) 1)))
  (switch `int` _output_get
    (:`0`
      (`KismetSystemLibrary.PrintString` "progress error!"))
    (:`1`
      (set `self.AircraftTargets` 2)
      (set `self.BaseTargets` 1)
      ;[1 1 1] generate combat 1 enemies
      (bind _outactors (`GameplayStatics.GetAllActorsOfClass` "/Game/Content_Level4/EnemyCharacter_Level4/BasicEnemy/BP_EnemyAircraftSpawnCombat1.BP_EnemyAircraftSpawnCombat1_C"))
      (for _array_element _outactors
        (`/Game/Content_Level4/EnemyCharacter_Level4/BasicEnemy/BP_EnemyAircraftSpawnCombat1.SpawnAnEnemy` _array_element))
      (bind _outactors_2 (`GameplayStatics.GetAllActorsOfClass` "/Game/Content_Level4/EnemyCharacter_Level4/BasicEnemy/Anti-Aircraft/BP_AntiAircraftSpawnCombat1.BP_AntiAircraftSpawnCombat1_C"))
      (for _array_element_2 _outactors_2
        (`/Game/Content_Level4/EnemyCharacter_Level4/BasicEnemy/Anti-Aircraft/BP_AntiAircraftSpawnCombat1.SpawnAnEnemy` _array_element_2))
      (bind _outactors_3 (`GameplayStatics.GetAllActorsOfClass` "/Game/Content_Level4/EnemyCharacter_Level4/AlienHome/BP_EnemyBaseSpawnCombat1.BP_EnemyBaseSpawnCombat1_C"))
      (for _array_element_3 _outactors_3
        (`/Game/Content_Level4/EnemyCharacter_Level4/AlienHome/BP_EnemyBaseSpawnCombat1.SpawnAnEnemy` _array_element_3))
      (set `self.CurrentEstimate` 0 :!label _label)
      (set `self.CurrentBaseEstimate` 0)
      (bind _outactors_4 (`GameplayStatics.GetAllActorsOfClass` "/Game/JetPlaneMap/Blueprints/BP_Airplane.BP_Airplane_C"))
      (bind _wbp_hud_main (`/Game/JetPlaneMap/Blueprints/BP_Airplane.WBP_HUD_Main` (`|GetArrayItem` _outactors_4)))
      (set `/Game/Content_Level4/UI/HUD/WBP_HUD_Main.AircraftsKilled` (`self.CurrentEstimate`) _wbp_hud_main)
      (set `/Game/Content_Level4/UI/HUD/WBP_HUD_Main.AircraftsToKill` (`self.AircraftTargets`) _wbp_hud_main)
      (set `/Game/Content_Level4/UI/HUD/WBP_HUD_Main.BasesDestroyed` (`self.CurrentBaseEstimate`) _wbp_hud_main)
      (set `/Game/Content_Level4/UI/HUD/WBP_HUD_Main.BasesToDestroy` (`self.BaseTargets`) _wbp_hud_main)
      (set `self.CanEnterNextProgress` false)
      (set `self.BaseEnemyClear` false)
      (set `self.AircraftEnemyClear` false))
    (:`2`
      (set `self.AircraftTargets` 2)
      (set `self.BaseTargets` 1)
      ;[1 1 1] generate combat 2 enemies
      (bind _outactors_5 (`GameplayStatics.GetAllActorsOfClass` "/Game/Content_Level4/EnemyCharacter_Level4/BasicEnemy/BP_EnemyAircraftSpawnCombat2.BP_EnemyAircraftSpawnCombat2_C"))
      (for _array_element_4 _outactors_5
        (`/Game/Content_Level4/EnemyCharacter_Level4/BasicEnemy/BP_EnemyAircraftSpawnCombat2.SpawnAnEnemy` _array_element_4))
      (bind _outactors_6 (`GameplayStatics.GetAllActorsOfClass` "/Game/Content_Level4/EnemyCharacter_Level4/BasicEnemy/Anti-Aircraft/BP_AntiAircraftSpawnCombat2.BP_AntiAircraftSpawnCombat2_C"))
      (for _array_element_5 _outactors_6
        (`/Game/Content_Level4/EnemyCharacter_Level4/BasicEnemy/Anti-Aircraft/BP_AntiAircraftSpawnCombat2.SpawnAnEnemy` _array_element_5))
      (bind _outactors_7 (`GameplayStatics.GetAllActorsOfClass` "/Game/Content_Level4/EnemyCharacter_Level4/AlienHome/BP_EnemyBaseSpawnCombat2.BP_EnemyBaseSpawnCombat2_C"))
      (for _array_element_6 _outactors_7
        (`/Game/Content_Level4/EnemyCharacter_Level4/AlienHome/BP_EnemyBaseSpawnCombat2.SpawnAnEnemy` _array_element_6))
      (goto _label))
    (:`3`
      (set `self.AircraftTargets` 2)
      (set `self.BaseTargets` 1)
      ;[1 1 1] generate combat 3 enemies
      (bind _outactors_8 (`GameplayStatics.GetAllActorsOfClass` "/Game/Content_Level4/EnemyCharacter_Level4/BasicEnemy/BP_EnemyAircraftSpawnCombat3.BP_EnemyAircraftSpawnCombat3_C"))
      (for _array_element_7 _outactors_8
        (`/Game/Content_Level4/EnemyCharacter_Level4/BasicEnemy/BP_EnemyAircraftSpawnCombat3.SpawnAnEnemy` _array_element_7))
      (bind _outactors_9 (`GameplayStatics.GetAllActorsOfClass` "/Game/Content_Level4/EnemyCharacter_Level4/BasicEnemy/Anti-Aircraft/BP_AntiAircraftSpawnCombat3.BP_AntiAircraftSpawnCombat3_C"))
      (for _array_element_8 _outactors_9
        (`/Game/Content_Level4/EnemyCharacter_Level4/BasicEnemy/Anti-Aircraft/BP_AntiAircraftSpawnCombat3.SpawnAnEnemy` _array_element_8))
      (bind _outactors_10 (`GameplayStatics.GetAllActorsOfClass` "/Game/Content_Level4/EnemyCharacter_Level4/AlienHome/BP_EnemyBaseSpawnCombat3.BP_EnemyBaseSpawnCombat3_C"))
      (for _array_element_9 _outactors_10
        (`/Game/Content_Level4/EnemyCharacter_Level4/AlienHome/BP_EnemyBaseSpawnCombat3.SpawnAnEnemy` _array_element_9))
      (goto _label))))

(fn `UpdateUIText`
  (bind _outactors (`GameplayStatics.GetAllActorsOfClass` "/Game/JetPlaneMap/Blueprints/BP_Airplane.BP_Airplane_C")))

(fn `UserConstructionScript`)