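; BP_EnemyBaseSpawnCombat3 is a spawn-point actor that creates a single BP_Outpost_New at its own location and rotation.
; A custom event calls SpawnAnEnemy when the triggering actor is exactly BP_Airplane, and a HasSpawned flag limits it to one spawn.
; The binding of that event to the first Trigger_End actor is disconnected and BeginPlay is empty, so nothing in this Blueprint hooks up the spawn.
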(event `self.ReceiveBeginPlay`)

(event `CustomEvent`
  (params (TriggerActor :type "Actor Object Reference"))
  (if (== (`GameplayStatics.GetObjectClass` TriggerActor) "/Game/JetPlaneMap/Blueprints/BP_Airplane.BP_Airplane_C")
    (`self.SpawnAnEnemy`)))

(fn `SpawnAnEnemy`
  (if (not (`self.HasSpawned`))
    (set `self.HasSpawned` true)
    (`KismetSystemLibrary.PrintString` "create enemy")
    (`|SpawnActorFromClass` "/Game/Content_Level4/EnemyCharacter_Level4/AlienHome/BP_Outpost_New.BP_Outpost_New_C" (`KismetMathLibrary.MakeTransform` (`self.K2_GetActorLocation`) (`self.K2_GetActorRotation`)) "AlwaysSpawn" "MultiplyWithRoot" null null)))

(fn `UserConstructionScript`)