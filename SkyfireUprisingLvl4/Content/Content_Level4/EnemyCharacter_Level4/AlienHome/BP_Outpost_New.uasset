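; BP_Outpost_New is an unfinished Level 4 alien outpost actor with four child-actor turret slots.
; BeginPlay casts each turret to BP_AAGun but does nothing with the result.
; TurretDestroyed prints a debug message and decrements TurretsRemaining, with nothing happening when it reaches zero.
; DamageActor is empty, and the health-loss and DestroyActor logic is disconnected, so the outpost never destroys itself.
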(event `DamageActor`)

(event `self.ReceiveBeginPlay`
  (for _array_element (`|MakeArray` (`self.Turret1`) (`self.Turret2`) (`self.Turret3`) (`self.Turret4`))
    (cast `/Game/Groundenemies/02/BP_AAGun` (`ChildActorComponent.ChildActor` _array_element))))

(event `TurretDestroyed`
  (`KismetSystemLibrary.PrintString` "DESTROYED TURRET")
  (set `self.TurretsRemaining` (- (`self.TurretsRemaining`) 1))
  (if (<= (`self.TurretsRemaining`) 0)
    _))

(fn `UserConstructionScript`)