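; Enemy aircraft that hunts the BP_Airplane player, registering with the game mode through BPI_EnemyManager and reporting when destroyed.
; A Tick state machine waits in Patrol, then cycles through Chase, Attack and Evade using timers, range and a facing check, firing one bullet per attack.
; Steering feeds interpolated pitch, yaw and roll into constant forward movement.
; Damage reveals fire effects, and death explodes the meshes into physics debris.
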(event `self.ReceiveBeginPlay`
  (bind _returnvalue (`GameplayStatics.GetGameMode`))
  ;[1 1 1] BeginPlay
  (`self.InitData`)
  (if (`KismetSystemLibrary.DoesImplementInterface` _returnvalue "/Game/Content_Level4/EnemyCharacter_Level4/BasicEnemy/BPI_EnemyManager.BPI_EnemyManager_C")
    (message `/Game/Content_Level4/EnemyCharacter_Level4/BasicEnemy/BPI_EnemyManager.RegisterEnemy` _returnvalue self)
    (else
      (`KismetSystemLibrary.PrintString` "interface failed"))))

(event `InitData`
  ;[1 1 1] InitData, set player
  (set `self.CurrentHP` (`self.MaxHP`))
  (set `self.CurrentSpeed` (`self.ThrustSpeed`))
  ;;[1 1 1] choose the player
  (bind _outactors (`GameplayStatics.GetAllActorsOfClass` "/Game/JetPlaneMap/Blueprints/BP_Airplane.BP_Airplane_C"))
  (set `self.Player` (`|GetArrayItem` _outactors))
  (`self.SetState` "NewEnumerator1")
  (`SceneComponent.SetVisibility` (`self.P_Fire`) false false)
  (`SceneComponent.SetVisibility` (`self.P_Fire1`) false false))

(event `self.ReceiveTick`
  (params (DeltaSeconds :type "Float (single-precision)"))
  ;[1 1 1] State Machine
  (switch `/Game/Content_Level4/EnemyCharacter_Level4/BasicEnemy/E_EnemyAircraftState` (`self.CurrentState`)
    (:`NewEnumerator1`
      (if (`self.IsDying`)
        (`self.SetState` "NewEnumerator5" :!label _label)
        (else
          (`self.PatrolState`))))
    (:`NewEnumerator3`
      (if (`self.IsDying`)
        (goto _label)
        (else
          (`self.Chase State`))))
    (:`NewEnumerator4`
      (if (`self.IsDying`)
        (goto _label)
        (else
          (`self.AttackState`))))
    (:`NewEnumerator0`
      (if (`self.IsDying`)
        (goto _label)
        (else
          (`self.EvadeState`))))
    (:`NewEnumerator5`
      (`self.DeadState`))))

(fn `Activate Explode VFX`
  (`SceneComponent.SetVisibility` (`self.P_Fire`) true false)
  (`SceneComponent.SetVisibility` (`self.P_Fire1`) true false)
  (`NiagaraFunctionLibrary.SpawnSystemAtLocation` "/Game/Content_Level4/Fab/MixedVFX/Particles/Explosions/NS_ExplosionMidAirBig.NS_ExplosionMidAirBig" (+ (`self.K2_GetActorLocation`) (* (`self.GetActorForwardVector`) 50.0)) (struct) (3.0 3.0 3.0)))

(fn `AttackState`
  (if (and (< (`KismetMathLibrary.VSize` (- (`self.K2_GetActorLocation` (`self.Player`)) (`self.K2_GetActorLocation`))) (`self.ForceEvadeRange`)) (not (`self.isDead`)))
    (`self.SetState` "NewEnumerator0")
    (else
      (`self.UpdatePosition` (`GameplayStatics.GetWorldDeltaSeconds`))
      (bind _output_get (set `self.DurationTime` (+ (`self.DurationTime`) (`GameplayStatics.GetWorldDeltaSeconds`))))
      (if (> _output_get (`self.AttackDuration`))
        (`self.ShootBullets`)
        (`self.SetState` "NewEnumerator0")))))

(fn `Chase State`
  (bind _returnvalue (`GameplayStatics.GetWorldDeltaSeconds`))
  (if (and (< (`KismetMathLibrary.VSize` (- (`self.K2_GetActorLocation` (`self.Player`)) (`self.K2_GetActorLocation`))) (`self.ForceEvadeRange`)) (not (`self.isDead`)))
    (`self.SetState` "NewEnumerator0")
    (else
      (bind (_pitch _yaw _roll) (`self.CalculateChaseInput` (`self.K2_GetActorLocation` (`self.Player`))))
      (`self.UpdatePitch` _returnvalue _pitch)
      (`self.UpdateYaw` _returnvalue _yaw)
      (`self.UpdateRoll` _returnvalue _roll)
      (`self.UpdatePosition` _returnvalue)
      ;[1 1 1] StateChange
      (bind _output_get (set `self.PlayerInFront` (> (`KismetMathLibrary.Dot_VectorVector` (`KismetMathLibrary.Normal` (`self.PositionToPlayer`)) (`self.GetActorForwardVector`)) 0.7)))
      (if (and _output_get (< (`self.DistanceToPlayer`) (`self.AttackRange`)))
        (bind _output_get_2 (set `self.AttackLockingTime` (+ (`self.AttackLockingTime`) (`GameplayStatics.GetWorldDeltaSeconds`))))
        (if (> _output_get_2 (`self.AttackTimeThreshold`))
          (`self.SetState` "NewEnumerator4"))
        (else
          (bind _output_get_3 (set `self.DurationTime` (- (`self.DurationTime`) (`GameplayStatics.GetWorldDeltaSeconds`))))
          (if (< _output_get_3 0.0)
            (`self.SetState` "NewEnumerator0")))))))

(fn `DeadState`
  (bind _returnvalue (`GameplayStatics.GetGameMode`))
  (if (`self.IsDying`)
    (`self.PlayExplosionSound`)
    (`PrimitiveComponent.SetCollisionEnabled` (`self.CollisionSphere`) "NoCollision")
    (`self.Activate Explode VFX`)
    (for _array_element (`self.K2_GetComponentsByClass` "/Script/Engine.StaticMeshComponent")
      (`PrimitiveComponent.SetSimulatePhysics` _array_element true)
      (`PrimitiveComponent.SetCollisionResponseToAllChannels` _array_element "ECR_Ignore")
      (`PrimitiveComponent.AddImpulse` _array_element (* (`KismetMathLibrary.RandomUnitVectorInConeInDegrees` (`self.GetActorForwardVector`) 40.0) 7000.0) "None" true))
    (set `self.IsDying` false)
    (set `self.isDead` true)
    (`self.SetLifeSpan` 5.0)
    (if (`KismetSystemLibrary.DoesImplementInterface` _returnvalue "/Game/Content_Level4/EnemyCharacter_Level4/BasicEnemy/BPI_EnemyManager.BPI_EnemyManager_C")
      (message `/Game/Content_Level4/EnemyCharacter_Level4/BasicEnemy/BPI_EnemyManager.RemoveEnemy` _returnvalue self)
      (message `/Game/Content_Level4/EnemyCharacter_Level4/BasicEnemy/BPI_EnemyManager.EnemyDestroy` _returnvalue)
      (else
        (`KismetSystemLibrary.PrintString` "interface failed")))))

(fn `EvadeState`
  (bind _returnvalue (`GameplayStatics.GetWorldDeltaSeconds`))
  (bind (_pitch _yaw _roll) (`self.CalculateChaseInput` (+ (`self.K2_GetActorLocation`) (`KismetMathLibrary.InverseTransformDirection` (`self.GetTransform`) (`self.EvadeDirection`)))))
  (`self.UpdatePitch` _returnvalue _pitch)
  (`self.UpdateYaw` _returnvalue _yaw)
  (`self.UpdateRoll` _returnvalue _roll)
  (`self.UpdatePosition` (`GameplayStatics.GetWorldDeltaSeconds`))
  (bind _output_get (set `self.DurationTime` (+ (`self.DurationTime`) (`GameplayStatics.GetWorldDeltaSeconds`))))
  (if (> _output_get (`self.NextEvadeDuration`))
    (`self.SetState` "NewEnumerator3")))

(fn `GetHit`
  (params (Damage :type Integer :default 1))
  (bind _output_get (set `self.CurrentHP` (- (`self.CurrentHP`) Damage)))
  (`KismetSystemLibrary.PrintString` (`KismetStringLibrary.Conv_IntToString` _output_get))
  (if (<= _output_get 0)
    (set `self.CurrentHP` 0))
  (switch `int` (`self.CurrentHP`)
    (:`Default`
      (set `self.IsDying` true :!label _label))
    (:`0`
      (goto _label))
    (:`1`
      (`SceneComponent.SetVisibility` (`self.P_Fire1`) true false))
    (:`2`
      (`SceneComponent.SetVisibility` (`self.P_Fire`) true false))))

(fn `GetPlayerPosition`)

(fn `GetRotateValues`
  (returns (YawInputValue :type "Float (double-precision)") (PitchInputValue :type "Float (double-precision)") (RollInputValue :type "Float (double-precision)"))
  (locals (YawValue :type "Float (double-precision)") (RollValue :type "Float (double-precision)") (PitchValue :type "Float (double-precision)") (DesiredDirection :type "Vector Structure"))
  (set `local.DesiredDirection` (`KismetMathLibrary.Normal` (- (`self.K2_GetActorLocation` (`self.Player`)) (`self.K2_GetActorLocation`))))
  (set `local.YawValue` (`KismetMathLibrary.FClamp` (`KismetMathLibrary.Dot_VectorVector` (`local.DesiredDirection`) (`SceneComponent.GetUpVector` (`self.Root`))) -1.0))
  (set `local.PitchValue` (`KismetMathLibrary.FClamp` (`KismetMathLibrary.Dot_VectorVector` (`local.DesiredDirection`) (`SceneComponent.GetRightVector` (`self.Root`))) -1.0))
  (return (`local.YawValue`) (`local.PitchValue`) (`KismetMathLibrary.FClamp` (* (`local.YawValue`) 0.7) -1.0)))

(fn `PatrolState`
  ;[1 1 1] Get Player Location
  (bind (_worldvectortoplayer _localvectortoplayer) (`self.GetLocateToPlayer` (`self.Player`)))
  (set `self.PositionToPlayer` _worldvectortoplayer)
  (set `self.RelativePositionToPlayer` _localvectortoplayer)
  ;[1 1 1] StateChange
  (if true
    (bind _output_get (set `self.DurationTime` (+ (`self.DurationTime`) (`GameplayStatics.GetWorldDeltaSeconds`))))
    (if (> _output_get (`self.StartChaseTime`))
      (`self.SetState` "NewEnumerator3"))
    (else
      (set `self.DurationTime` 0.0))))

(fn `PlayExplosionSound`
  (`GameplayStatics.PlaySoundAtLocation` "/Game/Content_Level4/Sounds/explosion.explosion" (`self.K2_GetActorLocation`) (struct) 1.0 1.0 0.0 null null null null))

(fn `SetState`
  (params (NewState :type "/Game/Content_Level4/EnemyCharacter_Level4/BasicEnemy/E_EnemyAircraftState Enum" :default "NewEnumerator1"))
  (bind _output_get (set `self.CurrentState` NewState))
  (switch `/Game/Content_Level4/EnemyCharacter_Level4/BasicEnemy/E_EnemyAircraftState` _output_get
    (:`NewEnumerator1`
      (set `self.DurationTime` 0.0))
    (:`NewEnumerator3`
      (set `self.DurationTime` (`KismetMathLibrary.RandomFloatInRange` 15.0 17.0))
      (set `self.AttackLockingTime` 0.0))
    (:`NewEnumerator4`
      (set `self.DurationTime` 0.0))
    (:`NewEnumerator0`
      (set `self.DurationTime` 0.0)
      (set `self.EvadeDirection` (`KismetMathLibrary.Normal` (`KismetMathLibrary.Cross_VectorVector` (- (`self.K2_GetActorLocation` (`self.Player`)) (`self.K2_GetActorLocation`)) (`KismetMathLibrary.RandomUnitVector`))))
      (set `self.NextEvadeDuration` (+ (`self.EvadeDuration`) (`KismetMathLibrary.RandomFloatInRange` 0.0 5.0))))))

(fn `ShootBullets`
  (`|SpawnActorFromClass` "/Game/Content_Level4/EnemyCharacter_Level4/BasicEnemy/BP_AircraftBullet.BP_AircraftBullet_C" (`KismetMathLibrary.MakeTransform` (`self.K2_GetActorLocation`) (`self.K2_GetActorRotation`) (5.0 5.0 5.0)) "Undefined" "MultiplyWithRoot" null null))

(fn `UpdatePitch`
  (params (DeltaSecond :type "Float (double-precision)") (ActionValue :type "Float (double-precision)"))
  ;[1 1 1] Get Target
  (set `self.TargetPitch` ActionValue)
  ;[1 1 1] Set Delta Yaw
  (bind _output_get (set `self.CurrentPitch` (`KismetMathLibrary.FInterpTo` (`self.CurrentPitch`) (`self.TargetPitch`) (`local.DeltaSecond`) 10.0)))
  ;[1 1 1] Rotate
  (`self.K2_AddActorLocalRotation` (`KismetMathLibrary.MakeRotator` 0.0 (* _output_get (`local.DeltaSecond`) (`self.PitchRotateSpeed`)))))

(fn `UpdatePosition`
  (params (DeltaSecond :type "Float (double-precision)"))
  ;[1 1 1] SetCurrentSpeed
  ;[1 1 1] ForwardPositionOffset
  (bind _output_get (set `self.NewPosition` (* (`self.GetActorForwardVector`) (* (`self.CurrentSpeed`) (`local.DeltaSecond`)))))
  ;[1 1 1] StallAndFallOffset
  (`self.K2_AddActorWorldOffset` _output_get)
  ;[1 1 1] Get Player Location
  (bind (_worldvectortoplayer _localvectortoplayer) (`self.GetLocateToPlayer` (`self.Player`)))
  (bind _output_get_2 (set `self.PositionToPlayer` _worldvectortoplayer))
  (set `self.RelativePositionToPlayer` _localvectortoplayer)
  (set `self.DistanceToPlayer` (`KismetMathLibrary.VSize` _output_get_2)))

(fn `UpdateRoll`
  (params (DeltaSecond :type "Float (double-precision)") (ActionValue :type "Float (double-precision)"))
  ;[1 1 1] Get Target
  (set `self.TargetRoll` ActionValue)
  ;[1 1 1] Set Delta Yaw
  (bind _output_get (set `self.CurrentRoll` (`KismetMathLibrary.FInterpTo` (`self.CurrentRoll`) (`self.TargetRoll`) (`local.DeltaSecond`) 10.0)))
  ;[1 1 1] Rotate
  (`self.K2_AddActorLocalRotation` (`KismetMathLibrary.MakeRotator` (* _output_get (`local.DeltaSecond`) (`self.RollRotateSpeed`)))))

(fn `UpdateYaw`
  (params (DeltaSecond :type "Float (double-precision)") (ActionValue :type "Float (double-precision)"))
  ;[1 1 1] Get Target
  (set `self.TargetYaw` ActionValue)
  ;[1 1 1] Set Delta Yaw
  (bind _output_get (set `self.CurrentYaw` (`KismetMathLibrary.FInterpTo` (`self.CurrentYaw`) (`self.TargetYaw`) (`local.DeltaSecond`) 10.0)))
  ;[1 1 1] Rotate
  (`self.K2_AddActorLocalRotation` (`KismetMathLibrary.MakeRotator` 0.0 0.0 (* _output_get (`local.DeltaSecond`) (`self.YawRotateSpeed`)))))

(fn `UserConstructionScript`)