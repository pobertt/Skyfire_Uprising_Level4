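; Flying enemy that chases player 0's pawn with plane-like movement.
; Each tick moves it along its forward vector, with gravity scaled by speed to mimic stalling.
; CalculateChaseInput turns the player's location into pitch, yaw and roll inputs, which are smoothed and applied as local rotations.
; Thrust control is unfinished: UpdateSpeed never runs, and GetRotateValues, an alternative dot-product steering calculation, is not called here.
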(event `self.ReceiveBeginPlay`
  ;[1 1 1] BeginPlay
  (`self.InitData`))

(event `InitData`
  ;[1 1 1] InitData, set player
  (bind _output_get (set `self.ThrustSpeed` (`self.MinThrustSpeed`)))
  (set `self.CurrentSpeed` _output_get)
  ;;[1 1 1] choose the player
  (set `self.Player` (`GameplayStatics.GetPlayerPawn` 0)))

(event `self.ReceiveTick`
  (params (DeltaSeconds :type "Float (single-precision)"))
  ;[1 1 1] UpdatePosition
  (`self.UpdatePosition` DeltaSeconds)
  (bind (_pitch _yaw _roll) (`self.CalculateChaseInput` (`self.K2_GetActorLocation` (`self.Player`))))
  (`self.UpdatePitch` (`GameplayStatics.GetWorldDeltaSeconds`) _pitch)
  (`self.UpdateYaw` (`GameplayStatics.GetWorldDeltaSeconds`) _yaw)
  (`self.UpdateRoll` (`GameplayStatics.GetWorldDeltaSeconds`) _roll))

(fn `GetPlayerPosition`)

(fn `GetRotateValues`
  (returns (YawInputValue :type "Float (double-precision)") (PitchInputValue :type "Float (double-precision)") (RollInputValue :type "Float (double-precision)"))
  (locals (YawValue :type "Float (double-precision)") (RollValue :type "Float (double-precision)") (PitchValue :type "Float (double-precision)") (DesiredDirection :type "Vector Structure"))
  (set `local.DesiredDirection` (`KismetMathLibrary.Normal` (- (`self.K2_GetActorLocation` (`self.Player`)) (`self.K2_GetActorLocation`))))
  (set `local.YawValue` (`KismetMathLibrary.FClamp` (`KismetMathLibrary.Dot_VectorVector` (`local.DesiredDirection`) (`SceneComponent.GetUpVector` (`self.Root`))) -1.0))
  (set `local.PitchValue` (`KismetMathLibrary.FClamp` (`KismetMathLibrary.Dot_VectorVector` (`local.DesiredDirection`) (`SceneComponent.GetRightVector` (`self.Root`))) -1.0))
  (return (`local.YawValue`) (`local.PitchValue`) (`KismetMathLibrary.FClamp` (* (`local.YawValue`) 0.7) -1.0)))

(fn `UpdatePitch`
  (params (DeltaSecond :type "Float (double-precision)") (ActionValue :type "Float (double-precision)"))
  ;[1 1 1] Get Target
  (set `self.TargetPitch` ActionValue)
  ;[1 1 1] Set Delta Yaw
  (bind _output_get (set `self.CurrentPitch` (`KismetMathLibrary.FInterpTo` (`self.CurrentPitch`) (`self.TargetPitch`) (`local.DeltaSecond`) 10.0)))
  ;[1 1 1] Rotate
  (`self.K2_AddActorLocalRotation` (`KismetMathLibrary.MakeRotator` 0.0 (* _output_get (`local.DeltaSecond`) (`self.PitchRotateSpeed`)))))

(fn `UpdatePosition`
  (params (DeltaSecond :type "Float (double-precision)"))
  (bind (_newposition_x _newposition_y _newposition_z) (`KismetMathLibrary.BreakVector` (`self.NewPosition`)))
  ;[1 1 1] SetCurrentSpeed
  (set `self.CurrentSpeed` (`KismetMathLibrary.SelectFloat` (`self.ThrustSpeed`) (`KismetMathLibrary.FInterpTo` (`self.CurrentSpeed`) (`self.ThrustSpeed`) (`local.DeltaSecond`) (`self.Drag`)) (< (`self.ThrustSpeed`) (`self.CurrentSpeed`))))
  ;[1 1 1] ForwardPositionOffset
  (set `self.NewPosition` (* (`self.GetActorForwardVector`) (* (`self.CurrentSpeed`) (`local.DeltaSecond`))))
  ;[1 1 1] StallAndFallOffset
  (set `self.AppliedGravity` (`KismetMathLibrary.MapRangeClamped` (`self.CurrentSpeed`) 0.0 (`self.MinThrustSpeed`) (`self.Gravity`)))
  (`self.K2_AddActorWorldOffset` (`KismetMathLibrary.MakeVector` _newposition_x _newposition_y (- _newposition_z (* (`self.AppliedGravity`) (`local.DeltaSecond`))))))

(fn `UpdateRoll`
  (params (DeltaSecond :type "Float (double-precision)") (ActionValue :type "Float (double-precision)"))
  ;[1 1 1] Get Target
  (set `self.TargetRoll` ActionValue)
  ;[1 1 1] Set Delta Yaw
  (bind _output_get (set `self.CurrentRoll` (`KismetMathLibrary.FInterpTo` (`self.CurrentRoll`) (`self.TargetRoll`) (`local.DeltaSecond`) 10.0)))
  ;[1 1 1] Rotate
  (`self.K2_AddActorLocalRotation` (`KismetMathLibrary.MakeRotator` (* _output_get (`local.DeltaSecond`) (`self.RollRotateSpeed`)))))

(fn `UpdateSpeed`
  (params (ActionValue :type "Float (double-precision)") (DeltaSecond :type "Float (double-precision)"))
  (locals (TargetThrustSpeed :type "Float (double-precision)"))
  ;[1 1 1] Acceletation
  (set `self.CurrentSpeed` (`KismetMathLibrary.FClamp` (+ (* ActionValue DeltaSecond (`self.Acceleration`)) (`self.CurrentSpeed`)) 0.0 (`self.MaxThrustSpeed`))))

(fn `UpdateYaw`
  (params (DeltaSecond :type "Float (double-precision)") (ActionValue :type "Float (double-precision)"))
  ;[1 1 1] Get Target
  (set `self.TargetYaw` ActionValue)
  ;[1 1 1] Set Delta Yaw
  (bind _output_get (set `self.CurrentYaw` (`KismetMathLibrary.FInterpTo` (`self.CurrentYaw`) (`self.TargetYaw`) (`local.DeltaSecond`) 10.0)))
  ;[1 1 1] Rotate
  (`self.K2_AddActorLocalRotation` (`KismetMathLibrary.MakeRotator` 0.0 0.0 (* _output_get (`local.DeltaSecond`) (`self.YawRotateSpeed`)))))

(fn `UserConstructionScript`)