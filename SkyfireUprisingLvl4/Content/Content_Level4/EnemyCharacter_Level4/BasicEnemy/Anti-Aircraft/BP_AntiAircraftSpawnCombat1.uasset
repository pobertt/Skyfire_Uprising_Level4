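; Spawner that places an anti-aircraft gun in the level when the player's airplane enters the first combat area.
; On BeginPlay it finds the first Trigger_Combat1 actor and binds to its enter-area event.
; When a BP_Airplane triggers it, a one-shot flag lets it spawn a BP_AAGun at its own location and rotation, ignoring collisions.
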(event `self.ReceiveBeginPlay`
  (bind _outactors (`GameplayStatics.GetAllActorsOfClass` "/Game/Level4/Trigger_Volume/Trigger_Combat1.Trigger_Combat1_C"))
  (add `/Game/Level4/Trigger_Volume/Trigger_Combat1.EnterArea` (`|GetArrayItem` _outactors) (delegate `CustomEvent`)))

(event `CustomEvent`
  (params (TriggerActor :type "Actor Object Reference"))
  (if (== (`GameplayStatics.GetObjectClass` TriggerActor) "/Game/JetPlaneMap/Blueprints/BP_Airplane.BP_Airplane_C")
    (`self.SpawnAnEnemy`)))

(fn `SpawnAnEnemy`
  (if (not (`self.HasSpawned`))
    (set `self.HasSpawned` true)
    (`KismetSystemLibrary.PrintString` "create enemy")
    (`|SpawnActorFromClass` "/Game/Groundenemies/02/BP_AAGun.BP_AAGun_C" (`KismetMathLibrary.MakeTransform` (`self.K2_GetActorLocation`) (`self.K2_GetActorRotation`)) "AlwaysSpawn" "MultiplyWithRoot" null null)))

(fn `UserConstructionScript`)