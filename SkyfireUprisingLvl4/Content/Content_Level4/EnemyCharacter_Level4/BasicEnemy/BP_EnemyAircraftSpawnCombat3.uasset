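; Level 4 spawn point that creates one BP_EnemyAircraft at its own location and rotation.
; Its EnterArea handler spawns the aircraft when the trigger actor is BP_Airplane and BP_GameMode_Level4 allows entering the next progress stage.
; A HasSpawned flag limits spawning to once.
; BeginPlay is empty, and the code binding EnterArea to the first Trigger_End actor is disconnected and never runs.
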(event `self.ReceiveBeginPlay`)

(event `EnterArea`
  (params (TriggerActor :type "Actor Object Reference"))
  (if (== (`GameplayStatics.GetObjectClass` TriggerActor) "/Game/JetPlaneMap/Blueprints/BP_Airplane.BP_Airplane_C")
    (bind _asbp_game_mode_level_4 (cast `/Game/Content_Level4/Gamemodes_Level4/BP_GameMode_Level4` (`GameplayStatics.GetGameMode`)))
    (if (`/Game/Content_Level4/Gamemodes_Level4/BP_GameMode_Level4.CanEnterNextProgress` _asbp_game_mode_level_4)
      (`self.SpawnAnEnemy`))))

(fn `SpawnAnEnemy`
  (if (not (`self.HasSpawned`))
    (set `self.HasSpawned` true)
    (`KismetSystemLibrary.PrintString` "create enemy")
    (`|SpawnActorFromClass` "/Game/Content_Level4/EnemyCharacter_Level4/BasicEnemy/BP_EnemyAircraft.BP_EnemyAircraft_C" (`KismetMathLibrary.MakeTransform` (`self.K2_GetActorLocation`) (`self.K2_GetActorRotation`)) "AlwaysSpawn" "MultiplyWithRoot" null null)))

(fn `UserConstructionScript`)