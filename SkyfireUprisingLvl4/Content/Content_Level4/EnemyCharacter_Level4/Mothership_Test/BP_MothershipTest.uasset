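; BP_MothershipTest is a test mothership that kills the player's airplane with an orbital laser strike when it leaves the map boundary.
; Exiting MapBoundary attaches a Niagara laser to the Sphere and plays the OrbitalStrike timeline, which updates the beam end to track the plane and drives its intensity.
; When the timeline finishes the plane dies; re-entering the boundary beforehand destroys the laser and stops the timeline.
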(event `self.MapBoundary.OnComponentEndOverlap`
  (params (OverlappedComponent :type "PrimitiveComponent Object Reference") (OtherActor :type "Actor Object Reference") (OtherComp :type "PrimitiveComponent Object Reference") (OtherBodyIndex :type Integer))
  (bind _bp_airplane (`self.BP_Airplane`))
  (bind _asbp_airplane (cast `/Game/JetPlaneMap/Blueprints/BP_Airplane` OtherActor))
  (set `self.BP_Airplane` _asbp_airplane)
  (bind _returnvalue (`NiagaraFunctionLibrary.SpawnSystemAttached` "/Game/Content_Level4/EnemyCharacter_Level4/Mothership_Test/NS_MothershipLaser.NS_MothershipLaser" (`self.Sphere`) "None" (0.0 0.0 0.0) (struct) "KeepRelativeOffset"))
  (set `self.ActiveLaser` _returnvalue)
  (bind (_direction _laserpower) (`Timeline|OrbitalStrike` :!via `PlayFromStart` :!label _label)
    (:`Update`
      (`/Engine/EditorBlueprintResources/StandardMacros.IsValid` (`self.ActiveLaser`)
        (:`Is Valid`
          (`NiagaraComponent.SetVariableVec3` (`self.ActiveLaser`) "BeamEnd" (`self.K2_GetActorLocation` (`self.BP_Airplane`)))
          (`NiagaraComponent.SetNiagaraVariableFloat` (`self.ActiveLaser`) "UserIntensity" _laserpower)
          (`KismetSystemLibrary.PrintString` (`KismetStringLibrary.Conv_DoubleToString` _laserpower) false))))
    (:`Finished`
      (`KismetSystemLibrary.PrintString` "finished")
      (set `/Game/JetPlaneMap/Blueprints/BP_Airplane.Health` 0.0 _bp_airplane)
      (`/Game/JetPlaneMap/Blueprints/BP_Airplane.Die` _bp_airplane "Death by Mothership"))))

(event `self.MapBoundary.OnComponentBeginOverlap`
  (params (OverlappedComponent :type "PrimitiveComponent Object Reference") (OtherActor :type "Actor Object Reference") (OtherComp :type "PrimitiveComponent Object Reference") (OtherBodyIndex :type Integer) (bFromSweep :type Boolean) (SweepResult :type "HitResult Structure (by ref)"))
  (bind _asbp_airplane (cast `/Game/JetPlaneMap/Blueprints/BP_Airplane` OtherActor))
  (set `self.BP_Airplane` _asbp_airplane)
  (`/Engine/EditorBlueprintResources/StandardMacros.IsValid` (`self.ActiveLaser`)
    (:`Is Valid`
      (`ActorComponent.K2_DestroyComponent` (`self.ActiveLaser`))
      (goto _label :!via `Stop`))))

(fn `UserConstructionScript`)