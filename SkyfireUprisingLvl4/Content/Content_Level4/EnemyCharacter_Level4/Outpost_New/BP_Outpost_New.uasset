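; BP_Outpost_New is a Level 4 enemy outpost that is destroyed once its turrets are gone.
; On BeginPlay it gives each of its four BP_AAGun child actors a reference back to itself.
; TurretDestroyed counts down the remaining turrets; at zero it notifies the outpost-tracking game mode and destroys the outpost.
; DamageActor is empty, and the health-based damage logic is disconnected.
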(event `DamageActor`)

(event `self.ReceiveBeginPlay`
  (for _array_element (`|MakeArray` (`self.Turret1`) (`self.Turret2`) (`self.Turret3`) (`self.Turret4`))
    (bind _asbp_aagun (cast `/Game/Groundenemies/02/BP_AAGun` (`ChildActorComponent.ChildActor` _array_element)))
    (set `/Game/Groundenemies/02/BP_AAGun.OutpostVar` self _asbp_aagun)))

(event `TurretDestroyed`
  (`KismetSystemLibrary.PrintString` "DESTROYED TURRET")
  (set `self.TurretsRemaining` (- (`self.TurretsRemaining`) 1))
  (if (<= (`self.TurretsRemaining`) 0)
    (bind _asbp_game_mode_level_4_outpost_tracking (cast `/Game/Content_Level4/Gamemodes_Level4/BP_GameMode_Level4_OutpostTracking` (`GameplayStatics.GetGameMode`)))
    (`/Game/Content_Level4/Gamemodes_Level4/BP_GameMode_Level4_OutpostTracking.OutpostDestroyed` _asbp_game_mode_level_4_outpost_tracking)
    (`self.K2_DestroyActor`)))

(fn `UserConstructionScript`)