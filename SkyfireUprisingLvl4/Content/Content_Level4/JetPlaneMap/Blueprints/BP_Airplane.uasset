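; BP_Airplane is a player-controlled airplane flown by applying physics forces to its static mesh.
; It adds the IMC_Airplane Enhanced Input context on begin play, with roll and pitch actions applying sensitivity-scaled torque around the mesh's forward and right axes.
; The power action sets a thrust value, printed for debugging and cleared on completion, which Tick applies as forward force.
; Torque and thrust both use acceleration change, making them mass-independent.
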(event `EnhancedInput|/Game/Content_Level4/JetPlaneMap/Inputs/IA_AirplaneRoll`
  (params (ActionValue :type "Float (double-precision)") (ElapsedSeconds :type "Float (double-precision)") (TriggeredSeconds :type "Float (double-precision)") (InputAction :type "InputAction Object Reference" :default "/Game/Content_Level4/JetPlaneMap/Inputs/IA_AirplaneRoll.IA_AirplaneRoll"))
  (bind _staticmesh (`self.StaticMesh`))
  ;[0.1615 0.1615 0.1615] Roll Action (X movement)
  (:`Triggered`
    (`PrimitiveComponent.AddTorqueInDegrees` _staticmesh (* ActionValue (`SceneComponent.GetForwardVector` _staticmesh) (`self.Sensitivity`)) "None" true)))

(event `EnhancedInput|/Game/Content_Level4/JetPlaneMap/Inputs/IA_AirplanePitch`
  (params (ActionValue :type "Float (double-precision)") (ElapsedSeconds :type "Float (double-precision)") (TriggeredSeconds :type "Float (double-precision)") (InputAction :type "InputAction Object Reference" :default "/Game/Content_Level4/JetPlaneMap/Inputs/IA_AirplanePitch.IA_AirplanePitch"))
  (bind _staticmesh (`self.StaticMesh`))
  ;[0.2156 0.2156 0.2156] Pitch Action (Y movement)
  (:`Triggered`
    (`PrimitiveComponent.AddTorqueInDegrees` _staticmesh (* ActionValue (`SceneComponent.GetRightVector` _staticmesh) (`self.Sensitivity`)) "None" true)))

(event `self.ReceiveBeginPlay`
  (`EnhancedInputSubsystemInterface.AddMappingContext` (pcsubsystem `EnhancedInputLocalPlayerSubsystem` (`GameplayStatics.GetPlayerController` 0)) "/Game/Content_Level4/JetPlaneMap/Inputs/IMC_Airplane.IMC_Airplane" 0 (struct)))

(event `EnhancedInput|/Game/Content_Level4/JetPlaneMap/Inputs/IA_AirplanePower`
  (params (ActionValue :type "Float (double-precision)") (ElapsedSeconds :type "Float (double-precision)") (TriggeredSeconds :type "Float (double-precision)") (InputAction :type "InputAction Object Reference" :default "/Game/Content_Level4/JetPlaneMap/Inputs/IA_AirplanePower.IA_AirplanePower"))
  (:`Triggered`
    (bind _output_get (set `self.Power` ActionValue))
    (`KismetSystemLibrary.PrintString` (`KismetStringLibrary.Conv_DoubleToString` (stale _output_get_2)) true true (struct :`G` 0.66 :`B` 1.0 :`A` 1.0) 0.0))
  (:`Completed`
    (bind _output_get_2 (set `self.Power` 0.0))))

(event `self.ReceiveTick`
  (params (DeltaSeconds :type "Float (single-precision)"))
  (bind _staticmesh (`self.StaticMesh`))
  (`PrimitiveComponent.AddForce` _staticmesh (* (`SceneComponent.GetForwardVector` _staticmesh) (`self.Power`)) "None" true))

(fn `UserConstructionScript`)