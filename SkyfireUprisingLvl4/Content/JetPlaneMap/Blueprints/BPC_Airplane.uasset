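; BPC_Airplane is an airplane Blueprint that tracks a throttle-like Power value.
; SetPower raises Power by PowerStep for positive input and lowers it by the same step otherwise, including at zero, clamping the result between zero and one.
; The event graph holds only a disabled BeginPlay, and nothing in the graphs applies Power to movement.
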(fn `SetPower`
  (params (PowerInput :type "Float (double-precision)"))
  (if (> PowerInput 0.0)
    (set `self.Power` (`KismetMathLibrary.FClamp` (+ (`self.Power`) (`self.PowerStep`))))
    (else
      (set `self.Power` (`KismetMathLibrary.FClamp` (- (`self.Power`) (`self.PowerStep`)))))))