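; Possessable physics-driven jet pawn with a machine gun and lock-on homing missiles.
; Enhanced Input applies pitch, roll and yaw torque and sets throttle flags; a looping timer ramps throttle, and Tick blends velocity toward the nose.
; A FOV-scaled sphere trace times HUD lock on "enemy" actors for BP_Missile, while the hitscan gun destroys them.
; Overlaps or hits at high throttle explode the plane and restart the level.
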(event `EnhancedInput|/Game/JetPlaneMap/Inputs/IA_PlaneRifle`
  (params (ActionValue :type Boolean) (ElapsedSeconds :type "Float (double-precision)") (TriggeredSeconds :type "Float (double-precision)") (InputAction :type "InputAction Object Reference" :default "/Game/JetPlaneMap/Inputs/IA_PlaneRifle.IA_PlaneRifle"))
  (bind _camera (`self.Camera`))
  ;[1 1 1] Rifle
  (:`Triggered`
    (set `self.MachineGun` true)
    (`/Engine/EditorBlueprintResources/StandardMacros.DoOnce` false :!label _label
      (:`Completed`
        (if (`self.MachineGun`)
          (`|ExecutionSequence`
            (:`then_0`
              (bind _outhit (`KismetSystemLibrary.LineTraceSingle` :`Start` (`SceneComponent.K2_GetComponentLocation` _camera) :`End` (* (`SceneComponent.GetForwardVector` _camera) 100000000.0) :`TraceChannel` "TraceTypeQuery1" :`DrawDebugType` "ForOneFrame"))
              (`|ExecutionSequence`
                (:`then_0`
                  (bind (_bblockinghit _binitialoverlap _time _distance _location _impactpoint _normal _impactnormal _physmat _hitactor) (`GameplayStatics.BreakHitResult` _outhit))
                  (`KismetSystemLibrary.PrintString` (`KismetSystemLibrary.GetDisplayName` _hitactor))
                  (if _bblockinghit
                    (if (`self.ActorHasTag` _hitactor "enemy")
                      (`self.K2_DestroyActor` _hitactor))))
                (:`then_1`
                  (`KismetSystemLibrary.Delay` 0.05)
                  (`|ExecutionSequence`
                    (:`then_0`
                      (goto _label :!via `Reset`))
                    (:`then_1`
                      (goto _label :!via `Reset`))))))
            (:`then_1`
              (`ActorComponent.Activate` (`self.RifleFireSound`) false)
              (`ActorComponent.Activate` (`self.MuzzleFlash`) false)))
          (else
            (goto _label :!via `Reset`))))))
  (:`Completed`
    (set `self.MachineGun` false)
    (`ActorComponent.Deactivate` (`self.MuzzleFlash`))
    (`ActorComponent.Deactivate` (`self.RifleFireSound`))))

(event `EnhancedInput|/Game/JetPlaneMap/Inputs/IA_PlaneRearView`
  (params (ActionValue :type Boolean) (ElapsedSeconds :type "Float (double-precision)") (TriggeredSeconds :type "Float (double-precision)") (InputAction :type "InputAction Object Reference" :default "/Game/JetPlaneMap/Inputs/IA_PlaneRearView.IA_PlaneRearView"))
  (:`Triggered`
    (`SceneComponent.K2_SetRelativeRotation` (`self.SpringArmCamera`) (struct :`Yaw` 180.0) false false))
  (:`Completed`
    (`SceneComponent.K2_SetRelativeRotation` :`self` (`self.SpringArmCamera`))))

(event `AddingForceInTick`
  (params (DeltaSeconds :type "Float (single-precision)"))
  ;[1 1 1] Adding Force
  (`|ExecutionSequence`
    (:`then_0`
      (`PrimitiveComponent.AddForce` (`self.CollisionBox`) (0.0 0.0 -1500.0) "None" true)
      (`self.Speed`))
    (:`then_1`
      (if (`self.ZeroThrottle`)
        (set `self.CurrentThrottle` (`KismetMathLibrary.FInterpTo_Constant` (`self.CurrentThrottle`) 0.0 (`GameplayStatics.GetWorldDeltaSeconds`) 1.0))))))

(event `EnhancedInput|/Game/JetPlaneMap/Inputs/IA_PlaneShooting`
  (params (ActionValue :type Boolean) (ElapsedSeconds :type "Float (double-precision)") (TriggeredSeconds :type "Float (double-precision)") (InputAction :type "InputAction Object Reference" :default "/Game/JetPlaneMap/Inputs/IA_PlaneShooting.IA_PlaneShooting"))
  (bind _returnvalue (`KismetMathLibrary.VSize` (`self.GetVelocity`)))
  ;[0.1865 0.1865 0.1865] Shooting Handler
  (:`Triggered`
    (`KismetSystemLibrary.PrintString` (`KismetStringLibrary.Conv_DoubleToString` _returnvalue) false true (struct :`R` 0.79156 :`B` 1.0 :`A` 1.0))
    (`|SpawnActorFromClass` "/Game/Content_Level4/Locking_Shooting/BP_Missile.BP_Missile_C" (`SceneComponent.K2_GetComponentToWorld` (`self.MissilePoint`)) "AlwaysSpawn" "MultiplyWithRoot" null (`self.CurrTarget`) (`/Game/Content_Level4/Locking_Shooting/UWB_HUD_LockOn.IsLockedOn` (`self.HUD_Circle_Ref`)) _returnvalue self)))

(event `self.ReceiveBeginPlay`
  ;[0.3115 0.3115 0.3115] Event Begin Play
  (`ActorComponent.Deactivate` (`self.NS_JetThruster_Level4_Left`))
  (`ActorComponent.Deactivate` (`self.NS_JetThruster_Level4_Right`))
  (bind _returnvalue (`|CreateWidget` "/Game/Content_Level4/Locking_Shooting/UWB_HUD_LockOn.UWB_HUD_LockOn_C"))
  (set `self.HUD_Circle_Ref` _returnvalue)
  (`KismetSystemLibrary.K2_SetTimer` null "Throttle" 0.025 true))

(event `EnhancedInput|/Game/JetPlaneMap/Inputs/IA_AirplaneRoll`
  (params (ActionValue :type "Float (double-precision)") (ElapsedSeconds :type "Float (double-precision)") (TriggeredSeconds :type "Float (double-precision)") (InputAction :type "InputAction Object Reference" :default "/Game/JetPlaneMap/Inputs/IA_AirplaneRoll.IA_AirplaneRoll"))
  ;[0.1615 0.1615 0.1615] Roll Action (X movement)
)

(event `self.ReceiveTick`
  (params (DeltaSeconds :type "Float (single-precision)"))
  ;[0.2448 0.2448 0.2448] Locking System
  (`self.AddingForceInTick` 0.0)
  (`self.SetWorldRadius`)
  (bind _start_vector (`self.GetSphereTraceStartVector`))
  (bind _end_vector (`self.GetSphereTraceEndVector`))
  (bind _outactors (`GameplayStatics.GetAllActorsWithTag` "ignore"))
  (bind _outhit (`KismetSystemLibrary.SphereTraceSingleForObjects` _start_vector _end_vector (`self.WorldRadius`) (`|MakeArray` "ObjectTypeQuery3" :!type "EObjectTypeQuery Enum") false _outactors "ForOneFrame"))
  (bind (_bblockinghit _binitialoverlap _time _distance _location _impactpoint _normal _impactnormal _physmat _hitactor) (`GameplayStatics.BreakHitResult` _outhit))
  (`self.PrintHitActor` _hitactor true)
  (if _bblockinghit
    (if (`self.ActorHasTag` _hitactor "enemy")
      (set `self.Hit Actor` _hitactor)
      (`self.EnemyHitHandler`)
      (else
        (set `/Game/Content_Level4/Locking_Shooting/UWB_HUD_LockOn.IsLockedOn` false (`self.HUD_Circle_Ref`) :!label _label_2)
        (set `self.LockTimer` 0.0)))
    (else
      (goto _label_2))))

(event `EnhancedInput|/Game/JetPlaneMap/Inputs/IA_AirplanePitch`
  (params (ActionValue :type "Float (double-precision)") (ElapsedSeconds :type "Float (double-precision)") (TriggeredSeconds :type "Float (double-precision)") (InputAction :type "InputAction Object Reference" :default "/Game/JetPlaneMap/Inputs/IA_AirplanePitch.IA_AirplanePitch"))
  ;[0.2156 0.2156 0.2156] Pitch Action (Y movement)
)

(event `InteractWithPlane`
  (params (`Player Controller` :type "PlayerController Object Reference"))
  ;[0.2573 0.2573 0.2573] Interaction With Plane
  (`Controller.Possess` `Player Controller` self)
  (`EnhancedInputSubsystemInterface.AddMappingContext` (pcsubsystem `EnhancedInputLocalPlayerSubsystem` (`GameplayStatics.GetPlayerController` 0)) "/Game/JetPlaneMap/Inputs/IMC_Airplane.IMC_Airplane" 0 (struct))
  (`UserWidget.AddToViewport` (`self.HUD_Circle_Ref`) 0)
  (`self.SetScaleFactorHUD`)
  (set `self.ZeroThrottle` true))

(event `EnhancedInput|/Game/JetPlaneMap/Inputs/IA_AirplaneYaw`
  (params (ActionValue :type "Float (double-precision)") (ElapsedSeconds :type "Float (double-precision)") (TriggeredSeconds :type "Float (double-precision)") (InputAction :type "InputAction Object Reference" :default "/Game/JetPlaneMap/Inputs/IA_AirplaneYaw.IA_AirplaneYaw"))
  ;[1 1 1] Yaw Movement
  (:`Triggered`
    (`PrimitiveComponent.AddTorqueInDegrees` (`self.CollisionBox`) (`KismetMathLibrary.VLerp` (0.0 0.0 0.0) (* (`SceneComponent.GetUpVector` (`self.CollisionBox`)) (* (* ActionValue 1250.0) (/ (`self.CurrentThrottle`) 750.0))) 0.1) "None" true)))

(event `EnhancedInput|/Game/JetPlaneMap/Inputs/IA_AirplanePower`
  (params (ActionValue :type "Float (double-precision)") (ElapsedSeconds :type "Float (double-precision)") (TriggeredSeconds :type "Float (double-precision)") (InputAction :type "InputAction Object Reference" :default "/Game/JetPlaneMap/Inputs/IA_AirplanePower.IA_AirplanePower"))
  ;[0.2198 0.2198 0.2198] Power Handler
)

(event `EnhancedInput|/Game/JetPlaneMap/Inputs/IA_AirplaneRoll`
  (params (ActionValue :type "Float (double-precision)") (ElapsedSeconds :type "Float (double-precision)") (TriggeredSeconds :type "Float (double-precision)") (InputAction :type "InputAction Object Reference" :default "/Game/JetPlaneMap/Inputs/IA_AirplaneRoll.IA_AirplaneRoll"))
  ;[1 1 1] Roll Movement
  (:`Triggered`
    (bind _output_get (set `self.MouseX` ActionValue))
    (bind _returnvalue (* _output_get -2000.0))
    (`PrimitiveComponent.AddTorqueInDegrees` (`self.CollisionBox`) (`KismetMathLibrary.VLerp` (0.0 0.0 0.0) (* (`SceneComponent.GetForwardVector` (`self.CollisionBox`)) (`KismetMathLibrary.SelectFloat` _returnvalue (/ _returnvalue 3.0) (> (`self.CurrentThrottle`) 0.0))) 0.1) "None" true)))

(event `Die`
  (bind _returnvalue (`GameplayStatics.GetPlayerController` 0))
  ;[1 1 1] Die
  (`GameplayStatics.SpawnEmitterAtLocation` "/Game/StarterContent/Particles/P_Explosion.P_Explosion" (`SceneComponent.K2_GetComponentLocation` (`self.CollisionBox`)) (struct) (20.0 20.0 20.0))
  (`self.DisableInput` _returnvalue null)
  (`self.SetActorHiddenInGame` _returnvalue true)
  (`self.SetActorHiddenInGame` self true)
  (`GameplayStatics.PlaySoundAtLocation` "/Engine/EngineSounds/1kSineTonePing.1kSineTonePing" (0.0 0.0 0.0) (struct) 1.0 1.0 0.0 null null null null)
  (`KismetSystemLibrary.Delay` 3.0)
  (`KismetSystemLibrary.ExecuteConsoleCommand` "RestartLevel" null))

(event `EnhancedInput|/Game/JetPlaneMap/Inputs/IA_AirplanePitch`
  (params (ActionValue :type "Float (double-precision)") (ElapsedSeconds :type "Float (double-precision)") (TriggeredSeconds :type "Float (double-precision)") (InputAction :type "InputAction Object Reference" :default "/Game/JetPlaneMap/Inputs/IA_AirplanePitch.IA_AirplanePitch"))
  (bind _returnvalue (* ActionValue -2000.0))
  ;[1 1 1] Pitch Movement
  (:`Triggered`
    (set `self.MouseY` ActionValue)
    (`PrimitiveComponent.AddTorqueInDegrees` (`self.CollisionBox`) (`KismetMathLibrary.VLerp` (0.0 0.0 0.0) (* (`SceneComponent.GetRightVector` (`self.CollisionBox`)) (`KismetMathLibrary.SelectFloat` _returnvalue (/ _returnvalue 3.0) (> (`self.CurrentThrottle`) 0.0))) 0.1) "None" true)))

(event `self.CollisionBox.OnComponentBeginOverlap`
  (params (OverlappedComponent :type "PrimitiveComponent Object Reference") (OtherActor :type "Actor Object Reference") (OtherComp :type "PrimitiveComponent Object Reference") (OtherBodyIndex :type Integer) (bFromSweep :type Boolean) (SweepResult :type "HitResult Structure (by ref)"))
  (if (`ActorComponent.ComponentHasTag` OtherComp "PlaneBody")
    _
    (elif (not (`self.ActorHasTag` OtherActor "MotherShip"))
      (`self.Die`))))

(event `EnhancedInput|/Game/JetPlaneMap/Inputs/IA_AirplanePower`
  (params (ActionValue :type "Float (double-precision)") (ElapsedSeconds :type "Float (double-precision)") (TriggeredSeconds :type "Float (double-precision)") (InputAction :type "InputAction Object Reference" :default "/Game/JetPlaneMap/Inputs/IA_AirplanePower.IA_AirplanePower"))
  ;[1 1 1] Power (W & S)
  (:`Triggered`
    (if (> ActionValue 0.0)
      (set `self.MoveThrottleUp` true)
      (set `self.ZeroThrottle` false)
      (set `self.MoveThrottleDown` false)
      (else
        (set `self.MoveThrottleUp` false)
        (set `self.ZeroThrottle` false)
        (set `self.MoveThrottleDown` true))))
  (:`Canceled`
    (set `self.MoveThrottleUp` false :!label _label_3)
    (set `self.ZeroThrottle` true)
    (set `self.MoveThrottleDown` false))
  (:`Completed`
    (goto _label_3)))

(event `self.ReceiveHit`
  (params (MyComp :type "PrimitiveComponent Object Reference") (Other :type "Actor Object Reference") (OtherComp :type "PrimitiveComponent Object Reference") (bSelfMoved :type Boolean) (HitLocation :type "Vector Structure") (HitNormal :type "Vector Structure") (NormalImpulse :type "Vector Structure") (Hit :type "HitResult Structure (by ref)"))
  (`KismetSystemLibrary.PrintString` "HIT" false)
  (if (>= (`self.CurrentThrottle`) 25.0)
    (`/Engine/EditorBlueprintResources/StandardMacros.DoOnce` false
      (:`Completed`
        (`self.Die`)))))

(fn `EnemyHitHandler`
  (if (== (`self.CurrTarget`) (`self.Hit Actor`))
    (bind _output_get (set `self.LockTimer` (+ (`self.LockTimer`) (`GameplayStatics.GetWorldDeltaSeconds`))))
    (set `/Game/Content_Level4/Locking_Shooting/UWB_HUD_LockOn.IsLockedOn` (>= _output_get (`self.LockOnMin`)) (`self.HUD_Circle_Ref`))
    (return)
    (else
      (set `self.CurrTarget` (`self.Hit Actor`))
      (set `self.LockTimer` 0.0))))

(fn `GetSphereTraceEndVector`
  (returns (`End Vector` :type "Vector Structure"))
  (bind _nosepoint (`self.NosePoint`))
  (return (+ (`SceneComponent.K2_GetComponentLocation` _nosepoint) (* (`SceneComponent.GetForwardVector` _nosepoint) (`self.TargetDistance`)))))

(fn `GetSphereTraceStartVector`
  (returns (`Start Vector` :type "Vector Structure"))
  (return (`SceneComponent.K2_GetComponentLocation` (`self.NosePoint`))))

(fn `PrintHitActor`
  (params (HitObject :type "Object Object Reference") (shouldPrint :type Boolean))
  (`KismetSystemLibrary.PrintString` (`KismetSystemLibrary.GetDisplayName` HitObject) false true (struct :`R` 0.989507 :`B` 1.0 :`A` 1.0))
  (return))

(fn `SetScaleFactorHUD`
  (bind (_x _y) (`KismetMathLibrary.BreakVector2D` (`WidgetLayoutLibrary.GetViewportSize`)))
  (set `self.ScaleVector` (/ (/ (`/Game/Content_Level4/Locking_Shooting/UWB_HUD_LockOn.CircleRadius` (`self.HUD_Circle_Ref`)) (/ _y 2.0)) (/ _x _y))))

(fn `SetWorldRadius`
  (set `self.WorldRadius` (* (`KismetMathLibrary.DegTan` (/ (`CameraComponent.FieldOfView` (`self.Camera`)) 2.0)) (`self.ScaleVector`) (`self.TargetDistance`))))

(fn `Speed`
  (bind _returnvalue (`PrimitiveComponent.GetPhysicsLinearVelocity` (`self.CollisionBox`) "None"))
  (`PrimitiveComponent.SetPhysicsLinearVelocity` (`self.CollisionBox`) (`KismetMathLibrary.VLerp` _returnvalue (* (`SceneComponent.GetForwardVector` (`self.CollisionBox`)) (* (`self.CurrentThrottle`) 500.0)) 0.1) false "None"))

(fn `Throttle`
  (`|ExecutionSequence`
    (:`then_0`
      (if (`self.MoveThrottleUp`)
        (set `self.CurrentThrottle` (`KismetMathLibrary.FClamp` (+ (`self.CurrentThrottle`) 0.1) 0.0 30.0))
        (`KismetSystemLibrary.PrintString` "THROTTLE" false)
        (elif (`self.MoveThrottleDown`)
          (set `self.CurrentThrottle` (`KismetMathLibrary.FClamp` (+ (`self.CurrentThrottle`) -1.0) 0.0 30.0)))))
    (:`then_1`
      (if (> (`self.CurrentThrottle`) 10.0)
        (`ActorComponent.Activate` (`self.NS_JetThruster_Level4_Right`) false)
        (`ActorComponent.Activate` (`self.NS_JetThruster_Level4_Left`) false)
        (else
          (`ActorComponent.Deactivate` (`self.NS_JetThruster_Level4_Left`))
          (`ActorComponent.Deactivate` (`self.NS_JetThruster_Level4_Right`)))))
    (:`then_2`
      (`KismetSystemLibrary.PrintString` "forsound" false))))

(fn `UserConstructionScript`)