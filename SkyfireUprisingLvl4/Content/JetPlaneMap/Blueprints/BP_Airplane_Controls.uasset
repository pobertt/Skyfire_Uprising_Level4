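; Player-pilotable jet plane that is possessed on interaction, flown with Enhanced Input and physics on its collision box.
; Pitch, roll and yaw apply torque against angular damping, while Tick adds downward force and blends velocity toward forward times throttle.
; A looping timer ramps throttle from held input and toggles thruster effects.
; Fast hits or overlaps, except tagged PlaneBody components or MotherShip actors, explode the plane and restart the level.
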(event `EnhancedInput|/Game/JetPlaneMap/Inputs/IA_AirplaneYaw`
  (params (ActionValue :type "Float (double-precision)") (ElapsedSeconds :type "Float (double-precision)") (TriggeredSeconds :type "Float (double-precision)") (InputAction :type "InputAction Object Reference" :default "/Game/JetPlaneMap/Inputs/IA_AirplaneYaw.IA_AirplaneYaw"))
  ;[1 1 1] Yaw Movement
  (:`Triggered`
    (`PrimitiveComponent.AddTorqueInDegrees` (`self.CollisionBox`) (`KismetMathLibrary.VLerp` (0.0 0.0 0.0) (* (`SceneComponent.GetUpVector` (`self.CollisionBox`)) (* (* ActionValue 1250.0) (/ (`self.CurrentThrottle`) 750.0))) 0.1) "None" true)))

(event `EnhancedInput|/Game/JetPlaneMap/Inputs/IA_AirplaneRoll`
  (params (ActionValue :type "Float (double-precision)") (ElapsedSeconds :type "Float (double-precision)") (TriggeredSeconds :type "Float (double-precision)") (InputAction :type "InputAction Object Reference" :default "/Game/JetPlaneMap/Inputs/IA_AirplaneRoll.IA_AirplaneRoll"))
  ;[1 1 1] Roll Movement
  (:`Triggered`
    (bind _output_get (set `self.MouseX` ActionValue))
    (bind _returnvalue (* _output_get -2000.0))
    (`PrimitiveComponent.AddTorqueInDegrees` (`self.CollisionBox`) (`KismetMathLibrary.VLerp` (0.0 0.0 0.0) (* (`SceneComponent.GetForwardVector` (`self.CollisionBox`)) (`KismetMathLibrary.SelectFloat` _returnvalue (/ _returnvalue 3.0) (> (`self.CurrentThrottle`) 0.0))) 0.1) "None" true)))

(event `self.ReceiveTick`
  (params (DeltaSeconds :type "Float (single-precision)"))
  (bind _collisionbox (`self.CollisionBox`))
  ;[1 1 1] Adding Force
  (`|ExecutionSequence`
    (:`then_0`
      (`PrimitiveComponent.AddTorqueInDegrees` _collisionbox (/ (`KismetMathLibrary.NegateVector` (`PrimitiveComponent.GetPhysicsAngularVelocityInDegrees` (`self.CollisionBox`) "None")) 0.75) "None" true)
      (`PrimitiveComponent.AddForce` _collisionbox (0.0 0.0 -1500.0) "None" true)
      (`self.Speed`))
    (:`then_1`
      (if (`self.ZeroThrottle`)
        (set `self.CurrentThrottle` (`KismetMathLibrary.FInterpTo_Constant` (`self.CurrentThrottle`) 0.0 (`GameplayStatics.GetWorldDeltaSeconds`) 1.0))))))

(event `EnhancedInput|/Game/JetPlaneMap/Inputs/IA_AirplanePitch`
  (params (ActionValue :type "Float (double-precision)") (ElapsedSeconds :type "Float (double-precision)") (TriggeredSeconds :type "Float (double-precision)") (InputAction :type "InputAction Object Reference" :default "/Game/JetPlaneMap/Inputs/IA_AirplanePitch.IA_AirplanePitch"))
  (bind _returnvalue (* ActionValue -2000.0))
  ;[1 1 1] Pitch Movement
  (:`Triggered`
    (set `self.MouseY` ActionValue)
    (`PrimitiveComponent.AddTorqueInDegrees` (`self.CollisionBox`) (`KismetMathLibrary.VLerp` (0.0 0.0 0.0) (* (`SceneComponent.GetRightVector` (`self.CollisionBox`)) (`KismetMathLibrary.SelectFloat` _returnvalue (/ _returnvalue 3.0) (> (`self.CurrentThrottle`) 0.0))) 0.1) "None" true)))

(event `self.ReceiveBeginPlay`
  (`KismetSystemLibrary.K2_SetTimer` null "Throttle" 0.025 true))

(event `EnhancedInput|/Game/JetPlaneMap/Inputs/IA_AirplanePower`
  (params (ActionValue :type "Float (double-precision)") (ElapsedSeconds :type "Float (double-precision)") (TriggeredSeconds :type "Float (double-precision)") (InputAction :type "InputAction Object Reference" :default "/Game/JetPlaneMap/Inputs/IA_AirplanePower.IA_AirplanePower"))
  ;[1 1 1] Power (W & S)
  (:`Triggered`
    (if (> ActionValue 0.0)
      (set `self.MoveThrottleUp` true)
      (set `self.ZeroThrottle` false)
      (set `self.MoveThrottleDown` false)
      (else
        (set `self.MoveThrottleUp` false)
        (set `self.ZeroThrottle` false)
        (set `self.MoveThrottleDown` true))))
  (:`Canceled`
    (set `self.MoveThrottleUp` false :!label _label)
    (set `self.ZeroThrottle` true)
    (set `self.MoveThrottleDown` false))
  (:`Completed`
    (goto _label)))

(event `InteractWithPlane`
  (params (`Player Controller` :type "PlayerController Object Reference"))
  ;[1 1 1] Interact
  (`Controller.Possess` `Player Controller` self)
  (`EnhancedInputSubsystemInterface.AddMappingContext` (pcsubsystem `EnhancedInputLocalPlayerSubsystem` (`GameplayStatics.GetPlayerController` 0)) "/Game/JetPlaneMap/Inputs/IMC_Airplane.IMC_Airplane" 0 (struct))
  (set `self.ZeroThrottle` true))

(event `self.ReceiveHit`
  (params (MyComp :type "PrimitiveComponent Object Reference") (Other :type "Actor Object Reference") (OtherComp :type "PrimitiveComponent Object Reference") (bSelfMoved :type Boolean) (HitLocation :type "Vector Structure") (HitNormal :type "Vector Structure") (NormalImpulse :type "Vector Structure") (Hit :type "HitResult Structure (by ref)"))
  (`KismetSystemLibrary.PrintString` "HIT" false)
  (if (>= (`self.CurrentThrottle`) 25.0)
    (`/Engine/EditorBlueprintResources/StandardMacros.DoOnce` false
      (:`Completed`
        (`self.Die`)))))

(event `self.CollisionBox.OnComponentBeginOverlap`
  (params (OverlappedComponent :type "PrimitiveComponent Object Reference") (OtherActor :type "Actor Object Reference") (OtherComp :type "PrimitiveComponent Object Reference") (OtherBodyIndex :type Integer) (bFromSweep :type Boolean) (SweepResult :type "HitResult Structure (by ref)"))
  (if (`ActorComponent.ComponentHasTag` OtherComp "PlaneBody")
    _
    (elif (not (`self.ActorHasTag` OtherActor "MotherShip"))
      (`self.Die`))))

(event `Die`
  (bind _returnvalue (`GameplayStatics.GetPlayerController` 0))
  (`GameplayStatics.SpawnEmitterAtLocation` "/Game/StarterContent/Particles/P_Explosion.P_Explosion" (0.0 0.0 0.0) (struct) (20.0 20.0 20.0))
  (`self.DisableInput` _returnvalue null)
  (`self.SetActorHiddenInGame` _returnvalue true)
  (`self.SetActorHiddenInGame` self true)
  (`GameplayStatics.PlaySoundAtLocation` "/Engine/EngineSounds/1kSineTonePing.1kSineTonePing" (0.0 0.0 0.0) (struct) 1.0 1.0 0.0 null null null null)
  (`KismetSystemLibrary.Delay` 3.0)
  (`KismetSystemLibrary.ExecuteConsoleCommand` "RestartLevel" null))

(fn `Speed`
  (bind _returnvalue (`PrimitiveComponent.GetPhysicsLinearVelocity` (`self.CollisionBox`) "None"))
  (`PrimitiveComponent.SetPhysicsLinearVelocity` (`self.CollisionBox`) (`KismetMathLibrary.VLerp` _returnvalue (* (`SceneComponent.GetForwardVector` (`self.CollisionBox`)) (* (`self.CurrentThrottle`) 500.0)) 0.1) false "None"))

(fn `Throttle`
  (`|ExecutionSequence`
    (:`then_0`
      (if (`self.MoveThrottleUp`)
        (set `self.CurrentThrottle` (`KismetMathLibrary.FClamp` (+ (`self.CurrentThrottle`) 0.1) 0.0 35.0))
        (elif (`self.MoveThrottleDown`)
          (set `self.CurrentThrottle` (`KismetMathLibrary.FClamp` (+ (`self.CurrentThrottle`) -1.0) 0.0 35.0)))))
    (:`then_1`
      (if (> (`self.CurrentThrottle`) 10.0)
        (`ActorComponent.Activate` (`self.NS_JetThruster_Level4_Right`) false)
        (`ActorComponent.Activate` (`self.NS_JetThruster_Level4_Left`) false)
        (else
          (`ActorComponent.Deactivate` (`self.NS_JetThruster_Level4_Left`))
          (`ActorComponent.Deactivate` (`self.NS_JetThruster_Level4_Right`)))))
    (:`then_2`
      (`KismetSystemLibrary.PrintString` "forsound" false))))

(fn `UserConstructionScript`)