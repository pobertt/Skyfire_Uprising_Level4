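; BP_Airplane is a possessable, physics-driven jet plane that the player flies after interacting with it.
; Interaction possesses the plane, adds its input mapping context and shows a lock-on HUD.
; Roll and pitch input apply acceleration-mode torque about the mesh's forward and right axes.
; Each power input raises an uncapped Power value, pushes the mesh forward and activates the twin thruster effects, which start off.
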(event `EnhancedInput|/Game/JetPlaneMap/Inputs/IA_AirplaneRoll`
  (params (ActionValue :type "Float (double-precision)") (ElapsedSeconds :type "Float (double-precision)") (TriggeredSeconds :type "Float (double-precision)") (InputAction :type "InputAction Object Reference" :default "/Game/JetPlaneMap/Inputs/IA_AirplaneRoll.IA_AirplaneRoll"))
  (bind _staticmesh (`self.StaticMesh`))
  ;[0.1615 0.1615 0.1615] Roll Action (X movement)
  (:`Triggered`
    (`PrimitiveComponent.AddTorqueInDegrees` _staticmesh (* ActionValue (`SceneComponent.GetForwardVector` _staticmesh) (`self.Sensitivity`)) "None" true)))

(event `EnhancedInput|/Game/JetPlaneMap/Inputs/IA_AirplanePitch`
  (params (ActionValue :type "Float (double-precision)") (ElapsedSeconds :type "Float (double-precision)") (TriggeredSeconds :type "Float (double-precision)") (InputAction :type "InputAction Object Reference" :default "/Game/JetPlaneMap/Inputs/IA_AirplanePitch.IA_AirplanePitch"))
  (bind _staticmesh (`self.StaticMesh`))
  ;[0.2156 0.2156 0.2156] Pitch Action (Y movement)
  (:`Triggered`
    (`PrimitiveComponent.AddTorqueInDegrees` _staticmesh (* ActionValue (`SceneComponent.GetRightVector` _staticmesh) (`self.Sensitivity`)) "None" true)))

(event `self.ReceiveBeginPlay`
  (`ActorComponent.Deactivate` (`self.NS_JetThruster_Level4_Left`))
  (`ActorComponent.Deactivate` (`self.NS_JetThruster_Level4_Right`)))

(event `self.ReceiveTick`
  (params (DeltaSeconds :type "Float (single-precision)")))

(event `EnhancedInput|/Game/JetPlaneMap/Inputs/IA_AirplanePower`
  (params (ActionValue :type "Vector2D Structure") (ElapsedSeconds :type "Float (double-precision)") (TriggeredSeconds :type "Float (double-precision)") (InputAction :type "InputAction Object Reference" :default "/Game/JetPlaneMap/Inputs/IA_AirplanePower.IA_AirplanePower"))
  (bind _staticmesh (`self.StaticMesh`))
  (:`Triggered`
    (bind _output_get (set `self.Power` (+ (`self.Power`) 20.0)))
    (`PrimitiveComponent.AddForce` _staticmesh (* (`SceneComponent.GetForwardVector` _staticmesh) (`self.Power`)) "None" true)
    (`KismetSystemLibrary.PrintString` (`KismetStringLibrary.Conv_DoubleToString` _output_get))
    (`ActorComponent.Activate` (`self.NS_JetThruster_Level4_Left`) false)
    (`ActorComponent.Activate` (`self.NS_JetThruster_Level4_Right`) false)))

(event `InteractWithPlane`
  (params (`Player Controller` :type "PlayerController Object Reference"))
  (`Controller.Possess` `Player Controller` self)
  (`EnhancedInputSubsystemInterface.AddMappingContext` (pcsubsystem `EnhancedInputLocalPlayerSubsystem` (`GameplayStatics.GetPlayerController` 0)) "/Game/JetPlaneMap/Inputs/IMC_Airplane.IMC_Airplane" 0 (struct))
  (bind _returnvalue (`|CreateWidget` "/Game/Content_Level4/Locking_Shooting/UWB_HUD_LockOn.UWB_HUD_LockOn_C"))
  (`UserWidget.AddToViewport` _returnvalue 0))

(fn `UserConstructionScript`)