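; BP_TestTarget is a test target actor that continuously drifts between random points.
; SetNewRandomTarget picks a point within MoveRange of the current location on X and Y, with an absolute height between HeightMin and HeightMax.
; Tick eases the actor toward that point with VInterpTo, without sweep, and picks a new one once it gets close.
; Ranges center on the current position, so it can wander away from its spawn.
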(event `self.ReceiveBeginPlay`
  (`self.SetNewRandomTarget`))

(event `self.ReceiveTick`
  (params (DeltaSeconds :type "Float (single-precision)"))
  (`self.K2_SetActorLocation` (`KismetMathLibrary.VInterpTo` (`self.K2_GetActorLocation`) (`self.MoveTargetLKocation`) DeltaSeconds 2.0))
  (if (< (`KismetMathLibrary.Vector_Distance` (`self.K2_GetActorLocation`) (`self.MoveTargetLKocation`)) 100.0)
    (`self.SetNewRandomTarget`)))

(fn `SetNewRandomTarget`
  (bind _moverange (`self.MoveRange`))
  (bind _moverange_2 (`self.MoveRange`))
  (bind _x (.x (`self.K2_GetActorLocation`)))
  (bind _y (.y (`self.K2_GetActorLocation`)))
  (set `self.MoveTargetLKocation` (`KismetMathLibrary.MakeVector` (`KismetMathLibrary.RandomFloatInRange` (- _x _moverange_2) (+ _x _moverange_2)) (`KismetMathLibrary.RandomFloatInRange` (- _y _moverange) (+ _y _moverange)) (`KismetMathLibrary.RandomFloatInRange` (`self.HeightMin`) (`self.HeightMax`)))))

(fn `UserConstructionScript`)