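; Anti-aircraft gun ground enemy that tracks the player pawn and fires bullets at it.
; On BeginPlay it plays a startup montage, then activates after a delay and starts a looping fire timer.
; Tick feeds aim yaw and pitch into ABP_AAGun, with pitch measured from a head socket.
; FIRE spawns BP_AABullet at each muzzle socket, offsetting the aim point by a velocity-based lead estimate.
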(event `self.ReceiveBeginPlay`
  ;[1 1 1] seekforplayer
  (bind _outactors (`GameplayStatics.GetAllActorsOfClass` "/Game/Groundenemies/02/BP_TestTarget.BP_TestTarget_C"))
  (set `self.TargetActor` (`GameplayStatics.GetPlayerPawn` 0))
  (`self.StartUp`))

(event `self.ReceiveTick`
  (params (DeltaSeconds :type "Float (single-precision)"))
  ;[1 1 1] rotation
  (if (`self.IsActivated`)
    (`/Engine/EditorBlueprintResources/StandardMacros.IsValid` (`self.TargetActor`)
      (:`Is Valid`
        (bind _asabp_aagun (cast `/Game/Groundenemies/02/ABP_AAGun` (`SkeletalMeshComponent.GetAnimInstance` (`self.AAGunMesh`))))
        (bind _output_get (set `/Game/Groundenemies/02/ABP_AAGun.AimYaw` (+ (.yaw (`KismetMathLibrary.FindLookAtRotation` (`self.K2_GetActorLocation`) (`self.K2_GetActorLocation` (`self.TargetActor`)))) 180.0) _asabp_aagun))
        (set `self.TargetLocation` (`self.K2_GetActorLocation` (`self.TargetActor`)))
        (bind _output_get_2 (set `self.HeadWorldTransform` (`SceneComponent.GetSocketTransform` (`self.AAGunMesh`) "Object180_0" "RTS_World")))
        (cast `/Game/Groundenemies/02/ABP_AAGun` (`SkeletalMeshComponent.GetAnimInstance` (`self.AAGunMesh`)))
        (set `/Game/Groundenemies/02/ABP_AAGun.AimPitch` (+ (.pitch (`KismetMathLibrary.MakeRotFromX` (`KismetMathLibrary.LessLess_VectorRotator` (`KismetMathLibrary.Normal` (- (`self.TargetLocation`) (.location _output_get_2))) (`KismetMathLibrary.MakeRotator` 0.0 0.0 _output_get)))) 0.0) _asabp_aagun)))))

(event `FIRE`
  (bind _returnvalue (`self.GetVelocity` (`self.TargetActor`)))
  ;[1 1 1] fire
  (if (`self.IsActivated`)
    (`/Engine/EditorBlueprintResources/StandardMacros.IsValid` (`self.TargetActor`)
      (:`Is Valid`
        (for _array_element (`self.MuzzleSockets`)
          (bind _returnvalue_2 (`SceneComponent.GetSocketLocation` (`self.AAGunMesh`) _array_element))
          (`|SpawnActorFromClass` "/Game/Groundenemies/02/BP_AABullet.BP_AABullet_C" (`KismetMathLibrary.MakeTransform` _returnvalue_2 (`KismetMathLibrary.FindLookAtRotation` _returnvalue_2 (+ (* _returnvalue (/ (`KismetMathLibrary.VSize` (- _returnvalue _returnvalue_2)) 3000.0)) (`self.TargetLocation`)))) "Undefined" "MultiplyWithRoot" null null))))))

(event `StartUp`
  (if (and (not (`self.IsStartingUp`)) (not (`self.IsActivated`)))
    (set `self.IsStartingUp` true)
    (`AnimInstance.Montage_Play` (`SkeletalMeshComponent.GetAnimInstance` (`self.AAGunMesh`)) "/Game/Groundenemies/02/AM_AAGun.AM_AAGun" 1.0 "MontageLength" 0.0 true)
    (`KismetSystemLibrary.Delay` 2.0)
    (`self.ActivateGun`)))

(event `ActivateGun`
  (set `self.IsStartingUp` false)
  (set `self.IsActivated` true)
  (`KismetSystemLibrary.K2_SetTimerDelegate` (`|CreateDelegate` :!event `FIRE`) 0.5 true))

(fn `UserConstructionScript`)